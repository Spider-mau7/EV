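; Base enemy Blueprint that exposes health, healing and damage functions by forwarding them to its BPCDmageSystem component.
; The construction script binds the component's death and block events, while the damage response binding sits unconnected.
; The attack event plays a montage on the mesh and calls OnAttackEnd on completion or interruption.
; Death, block and damage response handlers only print debug strings, and BeginPlay is empty.
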(event `self.ReceiveBeginPlay`)

(event `Attck`
  (`|PlayMontage` (`self.Mesh`) "/Game/Characters/Animaciones/Bailecito_Montage.Bailecito_Montage"
    (:`OnCompleted`
      _)
    (:`OnInterrupted`
      _))
  (`self.OnAttackEnd`))

(event `Death`
  (`KismetSystemLibrary.PrintString` "DAED"))

(event `bLOCKED`
  (params (CanBeParriedaram :type Boolean))
  (`KismetSystemLibrary.PrintString` "Blocked"))

(event `DamageRespone`
  (params (DamageResponse :type "/Game/DamageSystem/E_DamageResponse Enum" :default "NewEnumerator0"))
  (`KismetSystemLibrary.PrintString` (`|GetEnumeratorNameAsString` DamageResponse)))

(fn `GetCurrentHealth`
  (returns (Health :type "Float (double-precision)"))
  (return (`/Game/DamageSystem/BPC_DmageSystem.Healrh` (`self.BPC_DmageSystem`))))

(fn `GetMaxHealth`
  (returns (MaxHealth :type "Float (double-precision)"))
  (return (`/Game/DamageSystem/BPC_DmageSystem.MaxHealth` (`self.BPC_DmageSystem`))))

(fn `Heal`
  (params (Amount :type "Float (double-precision)"))
  (returns (NewHealth :type "Float (double-precision)"))
  (bind _newhealth (`/Game/DamageSystem/BPC_DmageSystem.Heal` (`self.BPC_DmageSystem`) Amount))
  (return _newhealth))

(fn `TakeDamage`
  (params (DamageInfo :type "/Game/DamageSystem/S_DamageInfo Structure"))
  (returns (WasDamaed :type Boolean))
  (bind _wasdamage (`/Game/DamageSystem/BPC_DmageSystem.TakeDamage` (`self.BPC_DmageSystem`) DamageInfo))
  (return _wasdamage))

(fn `UserConstructionScript`
  (bind _bpc_dmagesystem (`self.BPC_DmageSystem`))
  (add `/Game/DamageSystem/BPC_DmageSystem.OnDeath` _bpc_dmagesystem (`|CreateDelegate` :!event `Death`))
  (add `/Game/DamageSystem/BPC_DmageSystem.OnBlock` _bpc_dmagesystem (`|CreateDelegate` :!event `bLOCKED`)))